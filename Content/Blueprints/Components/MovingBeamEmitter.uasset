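; MovingBeamEmitter moves itself along the spline of an assigned Track; no beam logic appears in its graphs.
; On BeginPlay it caches and validates the Track's Spline, printing an error if either is missing.
; Otherwise the TweenMove timeline, with its play rate scaled by the inverse of Duration, drives Alpha, which maps to distance along the spline to set the root's world location.
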(event EventBeginPlay
  (CallFunction|Initialize)
  (if (Variables|Default|GetDependenciesOk)
    (|SetTimelineDuration)
    (bind _alpha (Timeline|TweenMove Play)
      (:Update
        (CallFunction|MoveSelf _alpha)))
    (else
      (Development|PrintString "Missing Dependency. Check that Component has Track assigned and that Track contains a Spline Component" true true "(R=0.000000,G=0.660000,B=1.000000,A=1.000000)" 5.0))))

(fn ConstructionScript
  (|CallParentFunction))

(fn MoveSelf
  (params (Alpha :type Float%20%28single-precision%29))
  (LocalVariables|SetLocal_Alpha Alpha)
  (Utilities|FlowControl|Sequence
    (:then_0
      (Variables|Default|SetDestination (Spline|GetLocationatDistanceAlongSpline (Variables|Default|GetSpline) (Math|Float|Lerp 0.0 (Spline|GetSplineLength (Variables|Default|GetSpline)) (LocalVariables|GetLocal_Alpha)) "World")))
    (:then_1
      (Transformation|SetWorldLocation (Variables|Default|GetDefaultSceneRoot) (Variables|Default|GetDestination) false false))))

(fn Initialize
  ;[1 1 1] Check dependencies and set them to variable
  (if (Utilities|IsValid (Variables|Default|GetTrack))
    (if (Utilities|IsValid (Variables|/Game/Blueprints/Components/Track.Track_C|GetSpline (Variables|Default|GetTrack)))
      (Variables|Default|SetSpline (Variables|/Game/Blueprints/Components/Track.Track_C|GetSpline (Variables|Default|GetTrack)))
      (else
        (Variables|Default|SetDependenciesOk false :!label _label)))
    (else
      (goto _label))))
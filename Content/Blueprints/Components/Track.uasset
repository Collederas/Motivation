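; Track moves a target actor along a spline over a configurable duration, starting at BeginPlay.
; Initialize caches the target's root component; its IsValid check is left unconnected, so dependencies are always marked OK.
; A timeline, with play rate set to the inverse of MoveDuration, drives MoveTarget each update.
; MoveTarget maps alpha to distance along the spline and sets the root's world location without sweeping.
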(event EventBeginPlay
  (CallFunction|Initialize)
  (|SetTimelineDuration)
  (bind _alpha (Timeline|MoveTween Play)
    (:Update
      (CallFunction|MoveTarget _alpha))))

(fn ConstructionScript)

(fn MoveTarget
  (params (Alpha :type Float%20%28single-precision%29))
  (LocalVariables|SetLocal_Alpha Alpha)
  (Utilities|FlowControl|Sequence
    (:then_0
      (Variables|Default|SetDestination (Spline|GetLocationatDistanceAlongSpline (Variables|Default|GetSpline) (Math|Float|Lerp 0.0 (Spline|GetSplineLength (Variables|Default|GetSpline)) (LocalVariables|GetLocal_Alpha)) "World")))
    (:then_1
      (Transformation|SetWorldLocation (Variables|Default|GetTargetRoot) (Variables|Default|GetDestination) false false))))

(fn Initialize
  ;[1 1 1] Check dependencies
  (if true
    (Variables|Default|SetDependenciesOk true)
    (Variables|Default|SetTargetRoot (Variables|/Script/Engine.Actor|GetRootComponent (Variables|Default|GetTarget)))))
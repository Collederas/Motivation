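; Scene component that makes its owning actor hover above surfaces by pushing it away from whatever lies beneath.
; On BeginPlay it caches the owner's first PrimitiveComponent as the body to push.
; Each tick it line-traces straight down in world space on the Visibility channel over TraceLength.
; A hit adds force along the impact normal, fading linearly to zero as distance approaches the trace length.
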(event EventTick
  (params (DeltaSeconds :type Float%20%28single-precision%29))
  (bind _returnvalue (Transformation|GetWorldLocation))
  (bind (_outhit _returnvalue_2) (Collision|LineTraceByChannel _returnvalue (- _returnvalue (Math|Vector|MakeVector 0.0 0.0 (Variables|Default|GetTraceLength))) "TraceTypeQuery1" false 0 "None"))
  (if _returnvalue_2
    (Physics|AddForce (Variables|Default|GetPrimitiveComponent) (* (.ImpactNormal (Collision|BreakHitResult _outhit)) (Math|Float|Lerp 5e+05 0.0 (/ (Math|Vector|VectorLength (- (.Location (Collision|BreakHitResult _outhit)) (Transformation|GetWorldLocation))) (Variables|Default|GetTraceLength)))) "None" false)))

(event EventBeginPlay
  (Variables|Default|SetPrimitiveComponent (Utilities|Array|Get(acopy) (Actor|GetComponentsByClass (Components|GetOwner) "/Script/Engine.PrimitiveComponent"))))
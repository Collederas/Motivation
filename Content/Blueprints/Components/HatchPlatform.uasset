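; Hatch platform Blueprint that swings open and closed when toggled, optionally opening itself at BeginPlay through OpenByDefault.
; Toggle runs TogglePlatform, which waits ActivationDelay, then plays or reverses the OpenClose timeline depending on IsOpen.
; The timeline's OpeningVector X drives the Platform's relative roll, with pitch and yaw held at zero.
; IsOpen changes only when the timeline finishes, alternating through a FlipFlop rather than reading the playback direction.
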(event Custom|Toggle
  (|TogglePlatform))

(event EventBeginPlay
  (if (Variables|Default|GetOpenByDefault)
    (CallFunction|Toggle)))

(fn ConstructionScript)
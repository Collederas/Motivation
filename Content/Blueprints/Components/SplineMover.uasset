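; SplineMover is a component that positions an actor along a spline.
; On BeginPlay it finds the SplineComponent on its owner and calls Move with an alpha of zero to target the start of the spline.
; Move maps the alpha to a distance along the spline's length, then sets OwnerRoot to that world location without sweep or teleport.
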(event EventBeginPlay
  (Utilities|FlowControl|Sequence
    (:then_0
      (Variables|Default|SetSpline (Actor|GetComponentbyClass (Components|GetOwner) "/Script/Engine.SplineComponent")))
    (:then_1
      (CallFunction|Move 0.0))))

(fn Move
  (params (Alpha :type Float%20%28single-precision%29) (Spline :type Spline%20Component%20Object%20Reference))
  (LocalVariables|SetLocal_Alpha Alpha)
  (Variables|Default|SetSpline Spline)
  (Utilities|FlowControl|Sequence
    (:then_0
      (LocalVariables|SetLocal_Destination (Spline|GetLocationatDistanceAlongSpline (Variables|Default|GetSpline) (Math|Float|Lerp 0.0 (Spline|GetSplineLength (Variables|Default|GetSpline)) (LocalVariables|GetLocal_Alpha)) "World")))
    (:then_1
      (Transformation|SetWorldLocation (Variables|Default|GetOwnerRoot) (LocalVariables|GetLocal_Destination) false false))))
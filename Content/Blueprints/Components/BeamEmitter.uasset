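; Beam emitter that works as a tripwire, toggling its connected platforms when a Pawn enters the beam.
; Each tick it recomputes start and end from the Emitter's location, forward vector and BeamDistance, then box-traces for Pawns with one-frame debug drawing.
; The AlreadyHit latch limits toggling to once per continuous hit and resets when the beam is clear.
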(event EventTick
  (params (DeltaSeconds :type Float%20%28single-precision%29))
  (Utilities|FlowControl|Sequence
    (:then_0
      (|SetEmissionVariables))
    (:then_1
      (bind _returnvalue (Class|KismetSystemLibrary|BoxTraceSingleforObjects (Variables|Default|GetStartLocation) (Variables|Default|GetEndLocation) (Variables|Default|GetColliderSize) "0, 0, 0" (Variables|Default|GetCollideWith) false 0 "ForOneFrame" true))
      (Variables|Default|SetIsHittingTarget _returnvalue))
    (:then_2
      (if (not (Variables|Default|GetIsHittingTarget))
        (Variables|Default|SetAlreadyHit false)))
    (:then_3
      (if (Variables|Default|GetIsHittingTarget)
        (if (not (Variables|Default|GetAlreadyHit))
          (for _array_element (Variables|Default|GetConnectedPlatforms)
            (Default|Toggle _array_element)
            (Variables|Default|SetAlreadyHit true)))))))

(fn ConstructionScript)
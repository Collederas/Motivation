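; Collectible reward actor that the first-person character picks up by pressing Interact while overlapping it.
; On BeginPlay it applies its Mesh variable and that mesh's first material to the Reward component.
; Overlap begin and end toggle the actor's input for player controller 0, so Interact only responds in range.
; Pickup prints the ObjectName in a message and destroys the actor, with no inventory or score update.
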(event EventTick
  (params (DeltaSeconds :type Float%20%28single-precision%29)))

(event Collision|EventActorBeginOverlap
  (params (OtherActor :type Actor%20Object%20Reference))
  (Utilities|Casting|CastToFirstPersonCharacter OtherActor)
  (Input|EnableInput (Game|GetPlayerController 0)))

(event Collision|EventActorEndOverlap
  (params (OtherActor :type Actor%20Object%20Reference))
  (Utilities|Casting|CastToFirstPersonCharacter OtherActor)
  (Input|DisableInput (Game|GetPlayerController 0)))

(event EventBeginPlay
  (bind _reward (Variables|Default|GetReward))
  (bind _mesh (Variables|Default|GetMesh))
  (Components|StaticMesh|SetStaticMesh _reward _mesh)
  (Rendering|Material|SetMaterial _reward 0 (Rendering|Material|GetMaterial _mesh 0)))

(event Input|ActionEvents|InputActionInteract
  (params (Key :type Key%20Structure :default "None"))
  (:Pressed
    (Development|PrintString (Utilities|String|ToString(Text) (Utilities|Text|FormatText "Picked up {Object Name}" (Variables|Default|GetObjectName))))
    (Utilities|FlowControl|Sequence
      (:then_0)
      (:then_1
        (Actor|DestroyActor)))))

(fn ConstructionScript)
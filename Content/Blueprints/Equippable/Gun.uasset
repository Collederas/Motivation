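; An equippable gun that vacuums up GunCollectible actors and stores their items in an inventory.
; Each tick it line-traces forward from the emission point, paused while the Fetch timeline plays, and toggles the collectible's highlight when hit state changes.
; Pressing Fire on a target adds its item to Inventory, disables collision and physics, then Fetch pulls it to the emission point, shrinking it before destroying it.
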(event EventBeginPlay
  (Input|EnableInput (Game|GetPlayerController 0)))

(event EventTick
  (params (DeltaSeconds :type Float%20%28single-precision%29))
  (Utilities|FlowControl|Sequence
    (:then_0
      (bind _output_get (Variables|Default|SetEmissionStart (Transformation|GetWorldLocation (Variables|Default|GetEmissionPoint))))
      (Variables|Default|SetEmissionEnd (+ (* (Math|Vector|GetForwardVector (Variables|Default|GetGun)) (Variables|Default|GetEmissionDistance)) _output_get)))
    (:then_1
      (if (not (Audio|Components|Audio|IsPlaying (Variables|Default|GetFetch)))
        (bind _outhit (Collision|LineTraceByChannel (Variables|Default|GetEmissionStart) (Variables|Default|GetEmissionEnd) "TraceTypeQuery1" false 0 "ForOneFrame"))
        (bind _asgun_collectible (Utilities|Casting|CastToGunCollectible (.HitActor (Collision|BreakHitResult _outhit)))
          (:then
            (Variables|Default|SetCollectible _asgun_collectible)
            (Variables|Default|SetIsHitting true))
          (:CastFailed
            (Variables|Default|SetIsHitting false)))))
    (:then_2
      (if (Variables|Default|GetIsHitting)
        (if (not (Variables|Default|GetAlreadyHit))
          (Class|GunCollectible|Highlight(Message) (Variables|Default|GetCollectible))
          (Variables|Default|SetAlreadyHit true))
        (elif (Variables|Default|GetAlreadyHit)
          (Class|GunCollectible|Highlight(Message) (Variables|Default|GetCollectible))
          (Variables|Default|SetAlreadyHit false))))))

(event Input|ActionEvents|InputActionFire
  (params (Key :type Key%20Structure :default "None"))
  (:Pressed
    (if (Variables|Default|GetIsHitting)
      (Utilities|FlowControl|Sequence
        (:then_0
          (Variables|Default|SetCollectibleMeshComponent (Actor|GetComponentbyClass (Variables|Default|GetCollectible) "/Script/Engine.StaticMeshComponent"))
          (bind _iteminstance (Class|GunCollectible|GetItem(Message) (Variables|Default|GetCollectible)))
          (Class|InventoryComponent|Add (Variables|Default|GetInventory) _iteminstance))
        (:then_1
          (Collision|SetActorEnableCollision (Variables|Default|GetCollectible) false)
          (Physics|SetSimulatePhysics (Variables|Default|GetCollectibleMeshComponent) false)
          (bind _duration (Timeline|Fetch PlayFromStart)
            (:Update
              (Transformation|SetActorLocation (Variables|Default|GetCollectible) (Math|Vector|Lerp(Vector) (Transformation|GetWorldLocation (Variables|Default|GetCollectibleMeshComponent)) (Transformation|GetWorldLocation (Variables|Default|GetEmissionPoint)) _duration) false false)
              (Transformation|SetActorScale3D (Variables|Default|GetCollectible) (Math|Vector|Lerp(Vector) (Transformation|GetActorScale3D (Variables|Default|GetCollectible)) "0, 0, 0" _duration)))
            (:Finished
              (Actor|DestroyActor (Variables|Default|GetCollectible)))))))))

(fn ConstructionScript)

(fn PickUp)

(fn GetItem
  (return 0))
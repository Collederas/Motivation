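; Construction-script generator that builds a hallway along an editable spline from deformed spline mesh components.
; It resizes HallwayDataArray to match the spline point count, giving each point its own settings entry.
; A loop over point indices calls BuildTrack, which stretches HallwayMesh to the next point using local locations and tangents.
; Where an entry's HasWindowR flag is set, WindowHallwayMesh is added over the same segment.
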(event EventBeginPlay)

(event Collision|EventActorBeginOverlap
  (params (OtherActor :type Actor%20Object%20Reference)))

(event EventTick
  (params (DeltaSeconds :type Float%20%28single-precision%29)))

(fn ConstructionScript
  (Utilities|FlowControl|Sequence
    (:then_0
      (|StoreNumberOfSplinePoints))
    (:then_1
      (|AddSplinePointsToArray))
    (:then_2
      (|ConstructLoop)
      (|StoreDrawMesh)
      (Utilities|FlowControl|Sequence
        (:then_0
          (CallFunction|BuildTrack (Variables|Default|GetCurrentIndexLoop) (Variables|Default|GetHallwayMesh)))
        (:then_1
          (if (Variables|Default|GetDrawWindow)
            (CallFunction|BuildTrack (Variables|Default|GetCurrentIndexLoop) (Variables|Default|GetWindowHallwayMesh))))))))

(fn BuildTrack
  (params (IndexLoop :type Integer) (ElementMesh :type Static%20Mesh%20Object%20Reference))
  (LocalVariables|SetLocal_CurrentLoopIndex IndexLoop)
  (LocalVariables|SetLocal_NextLoopIndex (+ IndexLoop 1))
  (LocalVariables|SetLocal_ElementMesh ElementMesh)
  (Utilities|FlowControl|Sequence
    (:then_0
      (LocalVariables|SetLocal_StartLocation (.Location (Spline|GetLocationandTangentatSplinePoint (Variables|Default|GetSpline) (LocalVariables|GetLocal_CurrentLoopIndex) "Local")))
      (LocalVariables|SetLocal_StartTangent (.Tangent (Spline|GetLocationandTangentatSplinePoint (Variables|Default|GetSpline) (LocalVariables|GetLocal_CurrentLoopIndex) "Local")))
      (LocalVariables|SetLocal_EndLocation (.Location (Spline|GetLocationandTangentatSplinePoint (Variables|Default|GetSpline) (LocalVariables|GetLocal_NextLoopIndex) "Local")))
      (LocalVariables|SetLocal_EndTangent (.Tangent (Spline|GetLocationandTangentatSplinePoint (Variables|Default|GetSpline) (LocalVariables|GetLocal_NextLoopIndex) "Local"))))
    (:then_1
      (bind _returnvalue (AddComponent|AddSplineMeshComponent false))
      (bind _output_get (LocalVariables|SetLocal_CurrentSplineMesh _returnvalue))
      (Components|StaticMesh|SetStaticMesh _output_get (LocalVariables|GetLocal_ElementMesh))
      (SplineMesh|SetStartandEnd (LocalVariables|GetLocal_CurrentSplineMesh) (LocalVariables|GetLocal_StartLocation) (LocalVariables|GetLocal_StartTangent) (LocalVariables|GetLocal_EndLocation) (LocalVariables|GetLocal_EndTangent) true :!class /Script/Engine.SplineMeshComponent))))
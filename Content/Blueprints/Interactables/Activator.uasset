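; Activator is an interactable actor that triggers a set of controlled objects when the player presses Interact nearby.
; Overlap begin and end with FirstPersonCharacter enable and disable its input from player controller 0, so the action only responds during overlap.
; On press, it converts ControlledObjects to an array and calls Activated on each entry.
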(event Collision|EventActorBeginOverlap
  (params (OtherActor :type Actor%20Object%20Reference))
  (Utilities|Casting|CastToFirstPersonCharacter OtherActor)
  (Input|EnableInput (Game|GetPlayerController 0)))

(event Collision|EventActorEndOverlap
  (params (OtherActor :type Actor%20Object%20Reference))
  (Utilities|Casting|CastToFirstPersonCharacter OtherActor)
  (Input|DisableInput (Game|GetPlayerController 0)))

(event Input|ActionEvents|InputActionInteract
  (params (Key :type Key%20Structure :default "None"))
  (:Pressed
    (bind _result (Utilities|Set|ToArray (Variables|Default|GetControlledObjects)))
    (for _array_element _result
      (Default|Activated _array_element))))

(fn ConstructionScript)
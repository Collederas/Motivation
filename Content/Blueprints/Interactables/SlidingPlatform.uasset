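; Sliding platform actor that moves its Platform component along a timeline when its Activated event fires.
; The Slide timeline plays when Active and reverses otherwise, with a FlipFlop on Finished toggling Active.
; Each update sets relative location to StartLocation plus the Sliding track, negating the whole sum unless Reversed is true.
; Debug prints show the actor location at BeginPlay and the target location during Reversed updates.
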(event Custom|Activated
  (if (Variables|Default|GetActive)
    (bind _sliding (Timeline|Slide Play)
      (:Update
        (if (Variables|Default|GetReversed)
          (Transformation|SetRelativeLocation (Variables|Default|GetPlatform) (+ (Variables|Default|GetStartLocation) _sliding) false false)
          (Development|PrintString (Utilities|String|ToString(Vector) (+ (Variables|Default|GetStartLocation) _sliding)))
          (else
            (Transformation|SetRelativeLocation (Variables|Default|GetPlatform) (* (+ (Variables|Default|GetStartLocation) _sliding) -1) false false))))
      (:Finished
        (Utilities|FlowControl|FlipFlop
          (:A
            (Variables|Default|SetActive false))
          (:B
            (Variables|Default|SetActive true)))))
    (else
      (Timeline|Slide Reverse))))

(event EventBeginPlay
  (Development|PrintString (Utilities|String|ToString(Vector) (Transformation|GetActorLocation))))

(fn ConstructionScript)
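; Elevator actor that travels up and down when its linked Switch is pressed.
; After a two-second delay, a timeline plays or reverses based on ArrivedUp, offsetting the platform's relative location from StartLocation.
; A FlipFlop toggles ArrivedUp each time the timeline finishes.
; A trigger enables input when the first-person character enters; the disable-input logic is disconnected, and Move is empty.
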(event OnComponentBeginOverlap(Trigger)
  (params (OverlappedComponent :type Primitive%20Component%20Object%20Reference) (OtherActor :type Actor%20Object%20Reference) (OtherComp :type Primitive%20Component%20Object%20Reference) (OtherBodyIndex :type Integer) (bFromSweep :type Boolean) (SweepResult :type Hit%20Result%20Structure%20%28by%20ref%29))
  ;[1 1 1] Handle Input
  (Utilities|Casting|CastToFirstPersonCharacter OtherActor)
  (Input|EnableInput (Game|GetPlayerController 0)))

(event OnComponentEndOverlap(Trigger)
  (params (OverlappedComponent :type Primitive%20Component%20Object%20Reference) (OtherActor :type Actor%20Object%20Reference) (OtherComp :type Primitive%20Component%20Object%20Reference) (OtherBodyIndex :type Integer))
  ;[1 1 1] Handle Input
)

(event Custom|Activate
  (params (Switch :type Elevator%20Switch%20Object%20Reference))
  (if (== Switch (Variables|Default|GetSwitch))
    (Utilities|FlowControl|Delay 2.0)
    (if (Variables|Default|GetArrivedUp)
      (bind _alhpa (Timeline|Up/Down Reverse)
        (:Update
          (Transformation|SetRelativeLocation (Variables|Default|GetElevator) (+ _alhpa (Variables|Default|GetStartLocation)) false false))
        (:Finished
          ;[1 1 1] Toggle
          (Utilities|FlowControl|FlipFlop
            (:A
              (Variables|Default|SetArrivedUp true))
            (:B
              (Variables|Default|SetArrivedUp false)))))
      (else
        (Timeline|Up/Down Play)))))

(event EventBeginPlay
  (EventDispatchers|BindEventtoSwitchPressed (Variables|Default|GetSwitch) (delegate Custom|Activate)))

(fn ConstructionScript)

(fn Move)
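; GunCollectible is a collectible world object that can optionally act as a projectile and supplies an item struct built from its display name.
; In projectile mode, construction sets initial speed and a custom collision channel and blocks pickup until the first Hit restores WorldStatic collision.
; Highlight, allowed only when pickupable, swaps the material and scales the mesh.
; Reset restores the material and scale cached at construction.
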(event EventReset
  (CallFunction|RestoreOriginalMaterial))

(event Collision|EventHit
  (params (MyComp :type Primitive%20Component%20Object%20Reference) (Other :type Actor%20Object%20Reference) (OtherComp :type Primitive%20Component%20Object%20Reference) (bSelfMoved :type Boolean) (HitLocation :type Vector :default "0, 0, 0") (HitNormal :type Vector :default "0, 0, 0") (NormalImpulse :type Vector :default "0, 0, 0") (Hit :type Hit%20Result%20Structure%20%28by%20ref%29))
  (Utilities|FlowControl|DoOnce false
    (:Completed
      (Collision|SetCollisionObjectType (Variables|Debug|GetStaticMeshComponent) "ECC_WorldStatic")
      (Variables|Default|SetCanBePickedUp true))))

(event EventHighlight
  (if (Variables|Default|GetCanBePickedUp)
    (CallFunction|SetHighlightProperties)))

(fn ConstructionScript
  (bind _staticmeshcomponent (Variables|Debug|GetStaticMeshComponent))
  (Utilities|FlowControl|Sequence
    (:then_0
      (Variables|Default|SetOriginalMaterial (Rendering|Material|GetMaterial _staticmeshcomponent 0))
      (Variables|Default|SetOriginalScale (Transformation|GetWorldScale _staticmeshcomponent)))
    (:then_1
      (bind _returnvalue (Class|Item|Make (Utilities|GetDisplayName self)))
      (Variables|Default|SetConstructedItem _returnvalue))
    (:then_2
      (if (Variables|Default|GetIsProjectile)
        (Variables|/Script/Engine.ProjectileMovementComponent|SetInitialSpeed (Variables|Default|GetProjectileMovement) (Variables|Default|GetInitialProjectileSpeed))
        (Collision|SetCollisionObjectType (Variables|Debug|GetStaticMeshComponent) "ECC_GameTraceChannel1")
        (Variables|Default|SetCanBePickedUp false)))))

(fn SetHighlightProperties
  (Utilities|FlowControl|Sequence
    (:then_0
      (Rendering|Material|SetMaterial (Variables|Debug|GetStaticMeshComponent) 0 "/Game/Art/Materials/Elevator.Elevator"))
    (:then_1
      (Transformation|SetRelativeScale3D (Variables|Debug|GetStaticMeshComponent) (* (Variables|Default|GetOriginalScale) (Variables|Default|GetHighlightScaleFactor))))
    (:then_2
      (Variables|Default|SetIsHighlighted true))))

(fn RestoreOriginalMaterial
  (bind _staticmeshcomponent (Variables|Debug|GetStaticMeshComponent))
  (Rendering|Material|SetMaterial _staticmeshcomponent 0 (Variables|Default|GetOriginalMaterial))
  (Variables|Default|SetIsHighlighted false)
  (Transformation|SetWorldScale3D _staticmeshcomponent (Variables|Default|GetOriginalScale)))

(fn GetItem
  (return (Variables|Default|GetConstructedItem)))
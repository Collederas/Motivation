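; Base sliding activatable actor that, on Activate, moves back and forth along a chosen world X, Y or Z axis by SlideAmount.
; The OpenClose timeline's alpha offsets the actor from the start location captured while inactive, with separate forward and reverse play rates.
; FlipFlops toggle Active when movement finishes, and AutoReverse sends the actor straight back.
; IsPlaying blocks re-activation mid-move, and debug prints report activation and start location.
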(event EventActivate
  (if (not (Variables|Default|GetIsPlaying))
    (Variables|Default|SetIsPlaying true)
    (Utilities|FlowControl|Sequence
      (:then_0
        (Development|PrintString (Utilities|String|ToString(Text) (Utilities|Text|FormatText "Activating {Actor}" self))))
      (:then_1
        (if (not (Variables|Default|GetActive))
          (bind _output_get (Variables|Default|SetStartLocation (Transformation|GetActorLocation)))
          (Development|PrintString (Utilities|String|ToString(Vector) _output_get))))
      (:then_2
        (bind _playrate (CallFunction|GetPlayRateforActiveState (Variables|Default|GetActive)))
        (Components|Timeline|SetPlayRate (Variables|Default|GetOpen/Close) _playrate)
        (if (Variables|Default|GetActive)
          (bind _alpha (Timeline|Open/Close Reverse)
            (:Update
              (bind _movementvector (CallFunction|GetMovementVector _alpha))
              (Transformation|SetActorLocation (+ (Variables|Default|GetStartLocation) _movementvector) false false))
            (:Finished
              (if (Variables|Default|GetAutoReverse)
                (|FlipFlopReverse)
                (else
                  (Utilities|FlowControl|FlipFlop
                    (:A
                      (Variables|Default|SetActive true))
                    (:B
                      (Variables|Default|SetActive false)))
                  (Variables|Default|SetIsPlaying false)))))
          (else
            (Timeline|Open/Close Play)))))))

(fn ConstructionScript)

(fn Reverse
  (bind _open_close (Variables|Default|GetOpen/Close))
  (Components|Timeline|SetPlayRate _open_close (Variables|Default|GetReversePlayRate))
  (Utilities|String|Reverse _open_close))

(fn GetMovementVector
  (params (Alpha :type Float%20%28single-precision%29))
  (bind _slideamount (Variables|Default|GetSlideAmount))
  (bind _returnvalue (* Alpha _slideamount))
  (switch Utilities|FlowControl|Switch|SwitchonAxisEnum (Variables|Default|GetSlideAxis)
    (:NewEnumerator0
      (Variables|Default|SetRelativeMovement (Math|Vector|MakeVector _returnvalue 0.0 0.0)))
    (:NewEnumerator1
      (Variables|Default|SetRelativeMovement (Math|Vector|MakeVector 0.0 _returnvalue 0.0)))
    (:NewEnumerator2
      (Variables|Default|SetRelativeMovement (Math|Vector|MakeVector 0.0 0.0 _returnvalue))))
  (return (Variables|Default|GetRelativeMovement)))

(fn GetPlayRateforActiveState
  (params (ActiveState :type Boolean))
  (if ActiveState
    (LocalVariables|SetReturnRate (Variables|Default|GetReversePlayRate))
    (else
      (LocalVariables|SetReturnRate (Variables|Default|GetPlayRate))))
  (return (LocalVariables|GetReturnRate)))
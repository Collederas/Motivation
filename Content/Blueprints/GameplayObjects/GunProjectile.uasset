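; GunProjectile is a gameplay object that can serve as a projectile and is flagged as pickupable after its first hit.
; When IsProjectile is set, construction applies the initial speed, a custom collision object type and disables pickup.
; The first hit switches collision to WorldStatic and enables pickup.
; Highlight swaps in the Elevator material while pickup is allowed, and Reset restores the material cached at construction.
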(event EventReset
  (CallFunction|RestoreOriginalMaterial))

(event Collision|EventHit
  (params (MyComp :type Primitive%20Component%20Object%20Reference) (Other :type Actor%20Object%20Reference) (OtherComp :type Primitive%20Component%20Object%20Reference) (bSelfMoved :type Boolean) (HitLocation :type Vector :default "0, 0, 0") (HitNormal :type Vector :default "0, 0, 0") (NormalImpulse :type Vector :default "0, 0, 0") (Hit :type Hit%20Result%20Structure%20%28by%20ref%29))
  (Utilities|FlowControl|DoOnce false
    (:Completed
      (Collision|SetCollisionObjectType (Variables|Default|GetStaticMeshComponent) "ECC_WorldStatic")
      (Variables|Default|SetCanBePickedUp true))))

(event EventHighlight
  (if (Variables|Default|GetCanBePickedUp)
    (CallFunction|SetHighlightProperties)))

(fn ConstructionScript
  (Utilities|FlowControl|Sequence
    (:then_0
      (Variables|Default|SetOriginalMaterial (Rendering|Material|GetMaterial (Variables|Default|GetStaticMeshComponent) 0)))
    (:then_1
      (if (Variables|Default|GetIsProjectile)
        (Variables|/Script/Engine.ProjectileMovementComponent|SetInitialSpeed (Variables|Default|GetProjectileMovement) (Variables|Default|GetProjectileInitialSpeed))
        (Collision|SetCollisionObjectType (Variables|Default|GetStaticMeshComponent) "ECC_GameTraceChannel1")
        (Variables|Default|SetCanBePickedUp false)))))

(fn SetHighlightProperties
  (Rendering|Material|SetMaterial (Variables|Default|GetStaticMeshComponent) 0 "/Game/Art/Materials/Elevator.Elevator")
  (Variables|Default|SetIsHighlighted true))

(fn RestoreOriginalMaterial
  (Rendering|Material|SetMaterial (Variables|Default|GetStaticMeshComponent) 0 (Variables|Default|GetOriginalMaterial))
  (Variables|Default|SetIsHighlighted false))
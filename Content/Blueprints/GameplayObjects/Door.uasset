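; Door actor that, when activated, moves vertically along a timeline, then automatically returns to where it started.
; The OpenClose timeline adds its ZLocation offset to the location captured on activation, without sweep.
; A FlipFlop on Finished alternates between marking it open and reversing at a separate play rate, and stopping once closed.
; An IsPlaying flag ignores further activations until the full cycle ends.
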(event EventActivate
  (if (not (Variables|Default|GetIsPlaying))
    (Variables|Default|SetIsPlaying true)
    (Utilities|FlowControl|Sequence
      (:then_0
        (Development|PrintString (Utilities|String|ToString(Text) (Utilities|Text|FormatText "Activating {Actor}" self))))
      (:then_1
        (Variables|Default|SetStartLocation (Transformation|GetActorLocation)))
      (:then_2
        (Components|Timeline|SetPlayRate (Variables|Default|GetOpen/Close) (Variables|Default|GetPlayRate))
        (bind _zlocation (Timeline|Open/Close Play)
          (:Update
            (Transformation|SetActorLocation (+ (Variables|Default|GetStartLocation) _zlocation) false false))
          (:Finished
            (|FlipFlopReverse)))))))

(fn ConstructionScript)
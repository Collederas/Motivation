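; Akey is a pickup actor, apparently a key, that adds itself to the player's inventory when overlapped.
; On any overlap it looks up an InventoryComponent on player character 0, without checking which actor overlapped.
; If the component exists, it passes its GetInventoryItem result to AddItem, prints the item name and a collection message, and destroys itself.
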(event Collision|EventActorBeginOverlap
  (params (OtherActor :type Actor%20Object%20Reference))
  (bind _returnvalue (Game|GetPlayerCharacter 0))
  (bind _returnvalue_2 (Actor|GetComponentbyClass _returnvalue "/Script/UnrealMotivation.InventoryComponent"))
  (Utilities|IsValid _returnvalue_2
    (:Is%20Valid
      (bind _returnvalue_3 (Class|Pickup|GetInventoryItem))
      (Development|PrintString (Utilities|String|ToString(Text) (Variables|/Script/UnrealMotivation.InventoryItem|GetName _returnvalue_3)))
      (Class|InventoryComponent|AddItem _returnvalue_2 _returnvalue_3)
      (Actor|DestroyActor)
      (Development|PrintText (Utilities|Text|FormatText "{Item} collected" 0)))))

(fn ConstructionScript)
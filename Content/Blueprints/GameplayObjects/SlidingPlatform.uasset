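; Sliding platform actor that moves between its start location and an offset along a chosen world X, Y or Z axis.
; The construction script builds the offset from axis and amount and scales the Slide timeline's play rate.
; Activate and Deactivate play or reverse the timeline, whose update lerps the platform's location without sweep.
; Toggle flips between them and, when Continuous is set, re-triggers itself after a delay for back-and-forth motion.
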(event EventActivate
  (params (Sender :type Actor%20Object%20Reference))
  (Audio|Components|Audio|Play (Variables|Default|GetSlide))
  (Variables|Default|SetIsActive true))

(event EventDeactivate
  (params (Sender :type Actor%20Object%20Reference))
  (Utilities|String|Reverse (Variables|Default|GetSlide))
  (Variables|Default|SetIsActive false))

(event EventToggle
  (params (Sender :type Actor%20Object%20Reference))
  (bind _self self)
  (if (Variables|Default|GetIsActive)
    (Class|ActivatableInterface|Deactivate _self)
    (else
      (Class|ActivatableInterface|Activate _self)))
  (if (Variables|Default|GetContinuous)
    (Utilities|FlowControl|Delay (Variables|Default|GetContinuousDelay))
    (Class|ActivatableInterface|Toggle)))

(event EventBeginPlay
  (Variables|Default|SetStartLocation (Transformation|GetWorldLocation (Variables|Default|GetPlatform))))

(fn ConstructionScript
  (bind _slidingamount (Variables|Default|GetSlidingAmount))
  (bind _slide (Variables|Default|GetSlide))
  (Utilities|FlowControl|Sequence
    (:then_0
      (switch Utilities|FlowControl|Switch|SwitchonAxisEnum (Variables|Default|GetSlidingAxis)
        (:NewEnumerator0
          (Variables|Default|SetSlideVector (Math|Vector|MakeVector _slidingamount 0.0 0.0)))
        (:NewEnumerator1
          (Variables|Default|SetSlideVector (Math|Vector|MakeVector 0.0 _slidingamount 0.0)))
        (:NewEnumerator2
          (Variables|Default|SetSlideVector (Math|Vector|MakeVector 0.0 0.0 _slidingamount)))))
    (:then_1
      (Components|Timeline|SetPlayRate _slide (* (Components|Animation|GetPlayRate _slide) (Variables|Default|GetSlideRate))))))
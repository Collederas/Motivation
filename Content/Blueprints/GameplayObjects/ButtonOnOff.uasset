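; A shootable on/off button that toggles when a GunProjectile overlaps it, with an optional key lock.
; An assigned KeyReference makes the Lock component start locked and supplies its key item on BeginPlay.
; Hits on a locked button try to unlock it using the player's InventoryComponent, printing a message on failure.
; Successful or unlocked hits call Toggle with the projectile, gated by a DoOnce that resets after a short delay.
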(event EventBeginPlay
  (CallFunction|SetKey))

(event Collision|EventActorBeginOverlap
  (params (OtherActor :type Actor%20Object%20Reference))
  (bind _asgun_projectile (Utilities|Casting|CastToGunProjectile OtherActor))
  (if (Variables|/Script/UnrealMotivation.LockComponent|GetLocked (Variables|Default|GetLock))
    (bind _inventory (CallFunction|GetPlayerInventory))
    (bind _returnvalue (Class|LockComponent|Unlock (Variables|Default|GetLock) _inventory))
    (if _returnvalue
      (Utilities|FlowControl|DoOnce false :!label _label
        (:Completed
          (Class|ActivatableInterface|Toggle _asgun_projectile)
          (Utilities|FlowControl|Delay 1.0)
          (goto _label Reset)))
      (else
        (Development|PrintString "Unlock Failed")))
    (else
      (goto _label))))

(fn ConstructionScript
  (bind _lock (Variables|Default|GetLock))
  (Utilities|IsValid (Variables|Default|GetKeyReference)
    (:Is%20Valid
      (Variables|/Script/UnrealMotivation.LockComponent|SetLocked _lock true))
    (:Is%20Not%20Valid
      (Variables|/Script/UnrealMotivation.LockComponent|SetLocked _lock false))))

(fn GetPlayerInventory
  (bind _returnvalue (Game|GetPlayerCharacter 0))
  (bind _returnvalue_2 (Actor|GetComponentbyClass _returnvalue "/Script/UnrealMotivation.InventoryComponent"))
  (Utilities|IsValid _returnvalue_2
    (:Is%20Valid
      (return _returnvalue_2))))

(fn SetKey
  (Utilities|IsValid (Variables|Default|GetKeyReference)
    (:Is%20Valid
      (bind _returnvalue (Class|Pickup|GetInventoryItem (Variables|Default|GetKeyReference)))
      (Variables|/Script/UnrealMotivation.LockComponent|SetKey (Variables|Default|GetLock) _returnvalue))))
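; Beam emitter actor whose collision box detects the first-person character, apparently intended to toggle connected platforms.
; BeginPlay passes BeamDistance to the particle system and adds it to the box's X extent.
; Overlap by the character reaches a switch on ActivationType with no actions attached.
; ToggleConnectedPlatforms toggles each linked platform, but its only calls sit in disconnected hit-check logic guarded by AlreadyHit.
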(event EventBeginPlay
  (Effects|Components|ParticleSystem|SetFloatParameter (Variables|Default|GetParticleSystem) "BeamDistance" (Variables|Default|GetBeamDistance))
  (Components|Box|SetBoxExtent (Variables|Default|GetCollisionArea) (+ (Variables|/Script/Engine.BoxComponent|GetBoxExtent (Variables|Default|GetCollisionArea)) (Math|Vector|MakeVector (Variables|Default|GetBeamDistance) 0.0 0.0)) true))

(event Collision|EventActorBeginOverlap
  (params (OtherActor :type Actor%20Object%20Reference))
  (Utilities|Casting|CastToFirstPersonCharacter OtherActor)
  (switch Utilities|FlowControl|Switch|SwitchonLaserActivationType (Variables|Default|GetActivationType)))

(fn ConstructionScript)

(fn ToggleConnectedPlatforms
  (for _array_element (Variables|Default|GetConnectedPlatforms)
    (Default|Toggle _array_element)))
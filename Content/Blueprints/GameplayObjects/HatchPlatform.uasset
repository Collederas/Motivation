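; HatchPlatform is a gameplay platform that swings open and closed like a hatch, optionally opening itself at BeginPlay.
; Activate waits an activation delay, sets the OpenClose timeline's play rate from the inverse of OpeningSpeed, then plays it from the start.
; The timeline drives the Platform's relative roll from a vector track's X value.
; Deactivate reverses the timeline immediately, with an IsOpen flag gating both events.
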(event Custom|Activate
  (if (not (Variables|Default|GetIsOpen))
    (Utilities|FlowControl|Delay (Variables|Default|GetActivationDelay))
    (Utilities|FlowControl|Sequence
      (:then_0
        (Components|Timeline|SetPlayRate))
      (:then_1
        (Components|Timeline|PlayfromStart (Variables|Default|GetOpen/Close))
        (Variables|Default|SetIsOpen true)))))

(event Custom|Deactivate
  (if (Variables|Default|GetIsOpen)
    (Utilities|String|Reverse (Variables|Default|GetOpen/Close))
    (Variables|Default|SetIsOpen false)))

(event EventBeginPlay
  (if (Variables|Default|GetOpenByDefault)
    (CallFunction|Activate)))

(fn ConstructionScript)
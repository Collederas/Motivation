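; Beam emitter puzzle actor that toggles its connected platforms when an actor enters the beam.
; Continuous mode toggles them again on exit, while Sequential mode leaves them switched.
; An overlapping Crate enables Tick, where a forward box trace shortens the particle beam and collision box to the hit distance.
; Overlap end stops Tick and, except for the first-person character, restores full beam length.
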(event EventBeginPlay
  (CallFunction|ResizeBeam (Variables|Default|GetBeamDistance))
  (Actor|Tick|SetActorTickEnabled false))

(event Collision|EventActorBeginOverlap
  (params (OtherActor :type Actor%20Object%20Reference))
  (CallFunction|ToggleConnectedPlatforms)
  (Utilities|Casting|CastToCrate OtherActor)
  (bind (_start _end) (CallFunction|GetTraceData))
  (Variables|Default|SetStartTrace _start)
  (Variables|Default|SetEndTrace _end)
  (Actor|Tick|SetActorTickEnabled true))

(event Collision|EventActorEndOverlap
  (params (OtherActor :type Actor%20Object%20Reference))
  (Actor|Tick|SetActorTickEnabled false)
  (switch Utilities|FlowControl|Switch|SwitchonLaserActivationType (Variables|Default|GetActivationType)
    (:NewEnumerator0
      _)
    (:NewEnumerator1
      (CallFunction|ToggleConnectedPlatforms)))
  (Utilities|Casting|CastToFirstPersonCharacter OtherActor
    (:CastFailed
      (CallFunction|ResizeBeam (Variables|Default|GetBeamDistance)))))

(event EventTick
  (params (DeltaSeconds :type Float%20%28single-precision%29))
  (bind _collisionarea (Variables|Default|GetCollisionArea))
  (bind _returnvalue (Components|Box|GetScaledBoxExtent _collisionarea))
  (bind _outhit (Collision|BoxTraceByChannel (Variables|Default|GetStartTrace) (Variables|Default|GetEndTrace) (Math|Vector|MakeVector (.y _returnvalue) (.y _returnvalue) (.z _returnvalue)) "0, 0, 0" "TraceTypeQuery1" false 0 "None"))
  (CallFunction|ResizeBeam (.Distance (Collision|BreakHitResult _outhit))))

(fn ConstructionScript)

(fn ToggleConnectedPlatforms
  (for _array_element (Variables|Default|GetConnectedPlatforms)
    (if (Variables|/Game/Blueprints/GameplayObjects/HatchPlatform.HatchPlatform_C|GetIsOpen _array_element)
      (Default|Deactivate _array_element)
      (else
        (Default|Activate _array_element)))))

(fn GetTraceData
  (bind _defaultsceneroot (Variables|Default|GetDefaultSceneRoot))
  (bind _returnvalue (Transformation|GetWorldLocation _defaultsceneroot))
  (bind _output_get (LocalVariables|SetStartTraceLocation _returnvalue))
  (bind _output_get_2 (LocalVariables|SetEndTraceLocation (+ _returnvalue (* (Math|Vector|GetForwardVector (Transformation|GetWorldRotation _defaultsceneroot)) (Variables|Default|GetBeamDistance)))))
  (return _output_get _output_get_2))

(fn ResizeBeam
  (params (Distance :type Float%20%28single-precision%29))
  (bind _output_get (LocalVariables|SetLocalDistance Distance))
  (Utilities|FlowControl|Sequence
    (:then_0
      (Effects|Components|ParticleSystem|SetFloatParameter (Variables|Default|GetParticleSystem) "BeamDistance" (LocalVariables|GetLocalDistance)))
    (:then_1
      (Components|Box|SetBoxExtent (Variables|Default|GetCollisionArea) (Math|Vector|MakeVector _output_get 32.0 32.0) true)
      (Transformation|SetRelativeLocation (Variables|Default|GetCollisionArea) (Math|Vector|MakeVector (/ (LocalVariables|GetLocalDistance) 2.0) 0.0 0.0) false false))))
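; Gun actor that sucks in GunProjectile collectibles and fires Crates from its muzzle.
; Tick line-traces forward from EmissionPoint, toggling the detected collectible's highlight message through DoOnce gates.
; Fire either pulls that collectible in with a shrinking timeline lerp and destroys it, or spawns a Crate, adding player X speed to launch speed.
; The construction script makes Inventory infinite with Crates; fetched objects are not added, and PickUp is empty.
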(event EventBeginPlay
  (Input|EnableInput (Game|GetPlayerController 0)))

(event EventTick
  (params (DeltaSeconds :type Float%20%28single-precision%29))
  (Utilities|FlowControl|Sequence
    (:then_0
      (bind _output_get (Variables|Default|SetEmissionStart (Transformation|GetWorldLocation (Variables|Default|GetEmissionPoint))))
      (Variables|Default|SetEmissionEnd (+ (* (Math|Vector|GetForwardVector (Variables|Default|GetGun)) (Variables|Default|GetEmissionDistance)) _output_get)))
    (:then_1
      (if (Variables|Default|GetPickUpState)
        (if (not (Audio|Components|Audio|IsPlaying (Variables|Default|GetFetchTimeline)))
          (bind _outhit (Collision|LineTraceByChannel (Variables|Default|GetEmissionStart) (Variables|Default|GetEmissionEnd) "TraceTypeQuery1" false 0 "ForOneFrame"))
          (bind _asgun_projectile (Utilities|Casting|CastToGunProjectile (.HitActor (Collision|BreakHitResult _outhit)))
            (:then
              (Variables|Default|SetIsDetectingCollectible true)
              (if (and (Utilities|IsValid (Variables|Default|GetCollectible)) (!= (Variables|Default|GetCollectible) (.HitActor (Collision|BreakHitResult _outhit))))
                (Class|GunProjectileInterface|Reset(Message) (Variables|Default|GetCollectible))
                (Variables|Default|SetCollectible _asgun_projectile)
                (Variables|Default|SetCollectibleChanged true)
                (else
                  (Variables|Default|SetCollectible _asgun_projectile)
                  (Variables|Default|SetCollectibleChanged false))))
            (:CastFailed
              (Variables|Default|SetIsDetectingCollectible false))))))
    (:then_2
      (if (Variables|Default|GetIsDetectingCollectible)
        (if (Variables|Default|GetCollectibleChanged)
          (goto _label Reset)
          (else
            (Utilities|FlowControl|DoOnce false :!label _label
              (:Completed
                (Utilities|IsValid (Variables|Default|GetCollectible)
                  (:Is%20Valid
                    (Class|GunProjectileInterface|Highlight(Message) (Variables|Default|GetCollectible))))))))
        (else
          (goto _label Reset))))
    (:then_3
      (if (Variables|Default|GetIsDetectingCollectible)
        (goto _label_2 Reset)
        (else
          (Utilities|FlowControl|DoOnce false :!label _label_2
            (:Completed
              (Utilities|IsValid (Variables|Default|GetCollectible)
                (:Is%20Valid
                  (Class|GunProjectileInterface|Reset(Message) (Variables|Default|GetCollectible)))))))))))

(event Input|ActionEvents|InputActionFire
  (params (Key :type Key%20Structure :default "None"))
  (:Pressed
    (if (Variables|Default|GetIsDetectingCollectible)
      (Variables|Default|SetIsDetectingCollectible false)
      (if (Variables|Default|GetPickUpState)
        (Utilities|FlowControl|Sequence
          (:then_0
            (Variables|Default|SetCollectibleMeshComponent (Actor|GetComponentbyClass (Variables|Default|GetCollectible) "/Script/Engine.StaticMeshComponent")))
          (:then_1
            (Collision|SetActorEnableCollision (Variables|Default|GetCollectible) false)
            (Physics|SetSimulatePhysics (Variables|Default|GetCollectibleMeshComponent) false)
            (bind _duration (Timeline|FetchTimeline PlayFromStart)
              (:Update
                (Variables|Default|SetPickUpState false)
                (Transformation|SetActorLocation (Variables|Default|GetCollectible) (Math|Vector|Lerp(Vector) (Transformation|GetWorldLocation (Variables|Default|GetCollectibleMeshComponent)) (Transformation|GetWorldLocation (Variables|Default|GetEmissionPoint)) _duration) false false)
                (Transformation|SetActorScale3D (Variables|Default|GetCollectible) (Math|Vector|Lerp(Vector) (Transformation|GetActorScale3D (Variables|Default|GetCollectible)) "0, 0, 0" _duration)))
              (:Finished
                (Actor|DestroyActor (Variables|Default|GetCollectible))
                (Variables|Default|SetPickUpState true))))))
      (else
        (CallFunction|Shoot)
        (Utilities|FlowControl|Delay 1.2)
        (Variables|Default|SetPickUpState true)))))

(fn ConstructionScript
  (bind _inventory (Variables|Default|GetInventory))
  (Variables|/Script/UnrealMotivation.InventoryComponent|SetInfiniteObjects _inventory true)
  (Variables|/Script/UnrealMotivation.InventoryComponent|SetInfiniteObjectsClass _inventory "/Game/Blueprints/GameplayObjects/Crate.Crate_C"))

(fn PickUp)

(fn Shoot
  (bind _returnvalue (Class|InventoryComponent|IsEmpty (Variables|Default|GetInventory)))
  (if _returnvalue
    (Development|PrintString "Empty Inventory")
    (else
      (bind _returnvalue_2 (Class|InventoryComponent|GetContent (Variables|Default|GetInventory)))
      (bind _returnvalue_3 (Game|SpawnActorfromClass "/Game/Blueprints/GameplayObjects/Crate.Crate_C" (Transformation|GetWorldTransform (Variables|Default|GetEmissionPoint)) "AlwaysSpawn" 0 true (+ (Math|Float|Absolute(Float) (.x (Pawn|Components|CharacterMovement|GetLastUpdateVelocity (Variables|/Script/Engine.Character|GetCharacterMovement (Game|GetPlayerCharacter 0))))) (Variables|Default|GetShootSpeed)) 0))
      (Class|InventoryComponent|RemoveItem (Variables|Default|GetInventory) (Utilities|Array|Get(acopy) _returnvalue_2 (Utilities|Array|LastIndex _returnvalue_2)))
      (Development|PrintText (Utilities|Text|FormatText "spawned {cltype}" _returnvalue_3)))))